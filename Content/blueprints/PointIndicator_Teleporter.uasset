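; Teleporter actor that moves anything overlapping its Capsule to an Arrow, which the construction script places from the Teleportlocation transform.
; It also means to align the player's control rotation, but compares the overlapped component to the player character, so that check likely never passes.
; A Cube overlap calls AddScore through a Player_Pawn cast, likewise made on the overlapped component instead of the other actor.
; A velocity reset is left unconnected.
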(event OnComponentBeginOverlap(Capsule)
  (params (OverlappedComponent :type Primitive%20Component%20Object%20Reference) (OtherActor :type Actor%20Object%20Reference) (OtherComp :type Primitive%20Component%20Object%20Reference) (OtherBodyIndex :type Integer) (bFromSweep :type Boolean) (SweepResult :type Hit%20Result%20Structure%20%28by%20ref%29))
  (bind _returnvalue (Game|GetPlayerCharacter 0))
  (Transformation|SetWorldTransform (Variables|/Script/Engine.Actor|GetRootComponent OtherActor) (Math|Transform|MakeTransform (.location (Transformation|GetWorldTransform (Variables|Default|GetArrow))) "0, 0, 0" "1,1,1") false false)
  (if (== OverlappedComponent _returnvalue)
    (Pawn|SetControlRotation (Game|GetPlayerController 0) (Transformation|GetActorRotation _returnvalue))))

(event OnComponentBeginOverlap(Cube)
  (params (OverlappedComponent :type Primitive%20Component%20Object%20Reference) (OtherActor :type Actor%20Object%20Reference) (OtherComp :type Primitive%20Component%20Object%20Reference) (OtherBodyIndex :type Integer) (bFromSweep :type Boolean) (SweepResult :type Hit%20Result%20Structure%20%28by%20ref%29))
  ;[1 1 1] Doesn't have a "primitive component?"
  (bind _asplayer_pawn (Utilities|Casting|CastToPlayer_Pawn OverlappedComponent))
  (Default|AddScore _asplayer_pawn))

(fn ConstructionScript
  (Transformation|SetRelativeTransform (Variables|Default|GetArrow) (Variables|Default|GetTeleportlocation) false false))