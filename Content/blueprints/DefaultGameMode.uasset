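; DefaultGameMode is a game mode that tracks the player's score and lives and sets up the on-screen HUD.
; BeginPlay creates the HUD widget for player controller 0 and adds it to the viewport.
; AddScore increments PlayerScore by one, while RemoveLife decrements PlayerLives and opens MainMenuLevel when lives reach exactly zero.
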(event EventBeginPlay
  (bind _returnvalue (UserInterface|CreateWidget "/Game/widgets/HUD.HUD_C" (Game|GetPlayerController 0)))
  (UserInterface|Viewport|AddtoViewport _returnvalue 0))

(event EventTick
  (params (DeltaSeconds :type Float%20%28single-precision%29)))

(fn ConstructionScript)

(fn AddScore
  (Variables|Default|SetplayerScore (+ (Variables|Default|GetplayerScore) 1)))

(fn RemoveLife
  (bind _output_get (Variables|Default|SetplayerLives (+ (Variables|Default|GetplayerLives) -1)))
  (if (== _output_get 0)
    (Game|OpenLevel(byName) "MainMenuLevel")))