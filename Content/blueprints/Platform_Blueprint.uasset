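; Moving platform that steps along negative X in the world and carries the player pawn with it.
; A looping one-second timer runs PlatformMove, which shifts the static mesh by a fixed offset, writing its world position back as a relative location.
; When PawnReference is valid and flags PlayerOnPlatform, the pawn's body and root are teleported by the same offset and the flag is cleared.
; Two identical macros perform the mesh step.
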(event EventBeginPlay
  (Utilities|Time|SetTimerbyFunctionName 0 "platformMove" 1.0 true))

(event EventTick
  (params (DeltaSeconds :type Float%20%28single-precision%29)))

(fn ConstructionScript)

(fn PlatformMove
  (bind _pawn_reference (Variables|Default|Getpawn_reference))
  (bind _pawn_reference_2 (Variables|Default|Getpawn_reference))
  (bind _defaultsceneroot (Variables|/Game/blueprints/Pawn_Blueprint.Pawn_Blueprint_C|GetDefaultSceneRoot _pawn_reference_2))
  (bind _returnvalue (Transformation|GetWorldLocation _defaultsceneroot))
  (bind (_x _y _z) (Math|Vector|BreakVector _returnvalue))
  (Utilities|IsValid _pawn_reference
    (:Is%20Valid
      (if (Variables|/Game/blueprints/Pawn_Blueprint.Pawn_Blueprint_C|GetplayerOnPlatform _pawn_reference)
        (Transformation|SetRelativeLocation (Variables|/Game/blueprints/Pawn_Blueprint.Pawn_Blueprint_C|GetamongusBody _pawn_reference_2) (Math|Vector|MakeVector (+ _x -2e+02) _y _z) false true)
        (Variables|/Game/blueprints/Pawn_Blueprint.Pawn_Blueprint_C|SetplayerOnPlatform (Variables|Default|Getpawn_reference) false)
        (|Movement_2_2)
        (else
          (|Movement_2 :!label _label))))
    (:Is%20Not%20Valid
      (goto _label))))