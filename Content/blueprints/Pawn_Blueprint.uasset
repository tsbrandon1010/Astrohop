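; Player pawn with an Among Us-style body that hops in fixed steps and tracks whether it is on a platform or the ground.
; Each WASD press offsets the body's world X or Y and writes it as relative location to root and body.
; Hits set or clear the platform flag, handing the pawn reference to Platform_Blueprint.
; Any overlap sets the ground flag, then passes the reference to floor_hitbox actors.
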(event EventBeginPlay)

(event Collision|EventActorBeginOverlap
  (params (OtherActor :type Actor%20Object%20Reference))
  (Variables|Default|SetplayerOnGround true)
  (bind _asfloor_hitbox (Utilities|Casting|CastTofloor_hitbox OtherActor))
  (Variables|/Game/blueprints/floor_hitbox.floor_hitbox_C|SetpawnReference _asfloor_hitbox self))

(event Collision|EventHit
  (params (MyComp :type Primitive%20Component%20Object%20Reference) (Other :type Actor%20Object%20Reference) (OtherComp :type Primitive%20Component%20Object%20Reference) (bSelfMoved :type Boolean) (HitLocation :type Vector :default "0, 0, 0") (HitNormal :type Vector :default "0, 0, 0") (NormalImpulse :type Vector :default "0, 0, 0") (Hit :type Hit%20Result%20Structure%20%28by%20ref%29))
  (if (== (Utilities|GetClass Other) "/Game/blueprints/Platform_Blueprint.Platform_Blueprint_C")
    (Variables|Default|SetplayerOnPlatform true)
    (bind _asplatform_blueprint (Utilities|Casting|CastToPlatform_Blueprint Other))
    (Variables|/Game/blueprints/Platform_Blueprint.Platform_Blueprint_C|Setpawn_reference _asplatform_blueprint self)
    (else
      (Variables|Default|SetplayerOnPlatform false))))

(event EventTick
  (params (DeltaSeconds :type Float%20%28single-precision%29)))

(fn ConstructionScript)

(event Input|ActionEvents|InputActionA_Left_Key
  (params (Key :type Key%20Structure))
  (bind _amongusbody (Variables|Default|GetamongusBody))
  (bind _returnvalue (Transformation|GetWorldLocation _amongusbody))
  (bind (_x _y _z) (Math|Vector|BreakVector _returnvalue))
  (:Pressed
    (Transformation|SetRelativeLocation (Variables|Default|GetDefaultSceneRoot) (Math|Vector|MakeVector (+ _x 2e+02) _y _z) false false)))

(event Input|ActionEvents|InputActionD_Right_Key
  (params (Key :type Key%20Structure))
  (bind _amongusbody (Variables|Default|GetamongusBody))
  (bind _returnvalue (Transformation|GetWorldLocation _amongusbody))
  (bind (_x _y _z) (Math|Vector|BreakVector _returnvalue))
  (:Pressed
    (Transformation|SetRelativeLocation (Variables|Default|GetDefaultSceneRoot) (Math|Vector|MakeVector (+ _x -2e+02) _y _z) false false)))

(event Input|ActionEvents|InputActionW_Forward_Key
  (params (Key :type Key%20Structure))
  (bind _amongusbody (Variables|Default|GetamongusBody))
  (bind _returnvalue (Transformation|GetWorldLocation _amongusbody))
  (bind (_x _y _z) (Math|Vector|BreakVector _returnvalue))
  (:Pressed
    (Transformation|SetRelativeLocation (Variables|Default|GetDefaultSceneRoot) (Math|Vector|MakeVector _x (+ _y 2e+02) _z) false false)))

(event Input|ActionEvents|InputActionS_Backwards_Key
  (params (Key :type Key%20Structure))
  (bind _amongusbody (Variables|Default|GetamongusBody))
  (bind _returnvalue (Transformation|GetWorldLocation _amongusbody))
  (bind (_x _y _z) (Math|Vector|BreakVector _returnvalue))
  (:Pressed
    (Transformation|SetRelativeLocation (Variables|Default|GetDefaultSceneRoot) (Math|Vector|MakeVector _x (+ _y -2e+02) _z) false false)))