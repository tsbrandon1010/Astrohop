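; Floor hitbox Blueprint that handles the penalty when the player hits the ground, returning them to spawn at the cost of a life.
; It polls the PlayerOnGround flag on a referenced pawn every Tick rather than handling an overlap itself.
; When the flag is set, it moves the pawn's AmongusBody and root to SpawnLocation, clears the flag and calls RemoveLife on DefaultGameMode.
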(event EventBeginPlay)

(event EventTick
  (params (DeltaSeconds :type Float%20%28single-precision%29))
  (bind _pawnreference (Variables|Default|GetpawnReference))
  (Utilities|IsValid _pawnreference
    (:Is%20Valid
      (if (Variables|/Game/blueprints/Pawn_Blueprint.Pawn_Blueprint_C|GetplayerOnGround _pawnreference)
        (Transformation|SetRelativeLocation (Variables|/Game/blueprints/Pawn_Blueprint.Pawn_Blueprint_C|GetamongusBody _pawnreference) (Variables|Default|GetspawnLocation) false false)
        (Variables|/Game/blueprints/Pawn_Blueprint.Pawn_Blueprint_C|SetplayerOnGround _pawnreference false)
        (bind _asdefault_game_mode (Utilities|Casting|CastToDefaultGameMode (Game|GetGameMode)))
        (Default|RemoveLife _asdefault_game_mode)))))

(fn ConstructionScript)